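; BP_Seva is an interactable actor, apparently pettable, that shows a W_Petting prompt while a player is inside its Sphere trigger.
; Overlap begin stores the player, lazily creates and displays the widget, and enables input; overlap end hides it and disables input.
; The F key toggles an Interacting flag through start and end events, and starting also hides the prompt.
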(event `self.Sphere.OnComponentBeginOverlap`
  (params (OverlappedComponent :type "PrimitiveComponent Object Reference") (OtherActor :type "Actor Object Reference") (OtherComp :type "PrimitiveComponent Object Reference") (OtherBodyIndex :type Integer) (bFromSweep :type Boolean) (SweepResult :type "HitResult Structure (by ref)"))
  (bind _yes_no (message `/Game/BP/BPI_Character.IsPlayer?` OtherActor))
  (if _yes_no
    (set `self.InteractingActor` OtherActor)
    (`self.WPetting`
      (:`then`
        _)
      (:`else`
        (bind _returnvalue (`|CreateWidget` "/Game/BP/W_Petting.W_Petting_C"))
        (set `self.WPetting` _returnvalue)))
    (`UserWidget.AddToViewport` (`self.WPetting`) 0)
    (`self.EnableInput` (`GameplayStatics.GetPlayerController` 0))))

(event `self.Sphere.OnComponentEndOverlap`
  (params (OverlappedComponent :type "PrimitiveComponent Object Reference") (OtherActor :type "Actor Object Reference") (OtherComp :type "PrimitiveComponent Object Reference") (OtherBodyIndex :type Integer))
  (bind _yes_no (message `/Game/BP/BPI_Character.IsPlayer?` OtherActor))
  (if _yes_no
    (`self.HideInstruction`)
    (`self.DisableInput` (`GameplayStatics.GetPlayerController` 0))))

(event `Key|F`
  (params (Key :type "Key Structure"))
  (:`Pressed`
    (if (`self.Interacting`)
      (`self.End Interaction`)
      (else
        (`self.Start Interaction`)))))

(event `Start Interaction`
  (set `self.Interacting` true)
  (`self.HideInstruction`))

(event `End Interaction`
  (set `self.Interacting` false))

(fn `UserConstructionScript`)