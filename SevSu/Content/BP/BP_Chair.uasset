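; Interactable chair Blueprint that lets an interacting Character sit down and stand up again.
; Starting interaction calls ToggleMovementMessage(false), plays SittingPose and eases the capsule onto the chair with MoveComponentTo, taking target yaw from the chair's location Z rather than its rotation.
; Ending interaction stops the montage, moves the character to StandLocation at its current rotation and calls ToggleMovementMessage(true).
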(event `self.Start Interaction`
  (bind (_returnvalue_x _returnvalue_y _returnvalue_z) (`KismetMathLibrary.BreakVector` (`self.K2_GetActorLocation`)))
  (bind _character (`self.Character`))
  (`parent.Start Interaction`)
  (bind _ascharacter (cast `Character` (`self.InteractingActor`)))
  (bind _output_get (set `self.Character` _ascharacter))
  (message `/Game/BP/BPI_Character.ToggleMovement` _output_get false)
  (`Character.PlayAnimMontage` _output_get "/Game/BP/ChairSitting/origs/SittingPose.SittingPose" 0.6 "None")
  (`KismetSystemLibrary.MoveComponentTo` (`Actor.RootComponent` _character) (+ (`self.K2_GetActorLocation`) (`KismetMathLibrary.MakeVector` 0.0 0.0 (`CapsuleComponent.CapsuleHalfHeight` (`Character.CapsuleComponent` _character)))) (`KismetMathLibrary.MakeRotator` 0.0 0.0 _returnvalue_z) true true 0.5))

(event `self.End Interaction`
  (bind _character (`self.Character`))
  (`parent.End Interaction`)
  (bind _character_2 (`self.Character`)
    (:`then`
      (`Character.StopAnimMontage` _character_2 "/Game/BP/ChairSitting/origs/SittingPose.SittingPose")
      (`KismetSystemLibrary.MoveComponentTo` (`Actor.RootComponent` _character) (+ (`SceneComponent.K2_GetComponentLocation` (`self.StandLocation`)) (`KismetMathLibrary.MakeVector` 0.0 0.0 (`CapsuleComponent.CapsuleHalfHeight` (`Character.CapsuleComponent` _character)))) (`self.K2_GetActorRotation` _character))
      (message `/Game/BP/BPI_Character.ToggleMovement` (`self.Character`) true))
    (:`else`)))

(fn `UserConstructionScript`
  (`parent.UserConstructionScript`))